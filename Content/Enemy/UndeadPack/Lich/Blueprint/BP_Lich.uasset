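; BP_Lich is the Lich enemy Blueprint, which alternates its patrol target between two patrol points.
; On BeginPlay it targets the first point, and overlapping either point switches the target to the other.
; Each change is written to the Blackboard as an object under PatrolPointKeyName, exposing the current destination to AI logic.
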(event EventBeginPlay
  (Variables|Default|SetCurrentPatrolPoint (Variables|Default|GetPatrolPoint1))
  (Utilities|UpdatePatrolPointBB))

(event Collision|EventActorBeginOverlap
  (params (OtherActor :type Actor%20Object%20Reference))
  (if (== OtherActor (Variables|Default|GetPatrolPoint1))
    (Variables|Default|SetCurrentPatrolPoint (Variables|Default|GetPatrolPoint2))
    (Utilities|UpdatePatrolPointBB :!label _label)
    (elif (== OtherActor (Variables|Default|GetPatrolPoint2))
      (Variables|Default|SetCurrentPatrolPoint (Variables|Default|GetPatrolPoint1))
      (goto _label))))

(event EventTick
  (params (DeltaSeconds :type Float%20%28single-precision%29)))

(fn ConstructionScript)