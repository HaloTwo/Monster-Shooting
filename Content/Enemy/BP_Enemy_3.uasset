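; BP_Enemy_3 is an enemy character that patrols between two points, damages the player and can be shot down.
; Overlapping either patrol point writes the other to the AI Blackboard; the initial-point setup is unconnected.
; Projectile hits drain health, spawn explosions and raise walk speed, until death animates, updates the player's kill count and goal check, then destroys the actor.
; Both hand components damage the player on overlap.
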(event OnComponentBeginOverlap(RightHand)
  (params (OverlappedComponent :type Primitive%20Component%20Object%20Reference) (OtherActor :type Actor%20Object%20Reference) (OtherComp :type Primitive%20Component%20Object%20Reference) (OtherBodyIndex :type Integer) (bFromSweep :type Boolean) (SweepResult :type Hit%20Result%20Structure%20%28by%20ref%29))
  (bind _asue_4asp_character (Utilities|Casting|CastToUe4ASP_Character OtherActor))
  (Game|Damage|ApplyDamage _asue_4asp_character 0.08 0 0))

(event OnComponentBeginOverlap(LiftHand)
  (params (OverlappedComponent :type Primitive%20Component%20Object%20Reference) (OtherActor :type Actor%20Object%20Reference) (OtherComp :type Primitive%20Component%20Object%20Reference) (OtherBodyIndex :type Integer) (bFromSweep :type Boolean) (SweepResult :type Hit%20Result%20Structure%20%28by%20ref%29))
  (bind _asue_4asp_character (Utilities|Casting|CastToUe4ASP_Character OtherActor))
  (Game|Damage|ApplyDamage _asue_4asp_character 0.08 0 0))

(event EventBeginPlay)

(event Collision|EventActorBeginOverlap
  (params (OtherActor :type Actor%20Object%20Reference))
  (if (== OtherActor (Variables|Default|GetPatrolPoint1))
    (Variables|Default|SetCurrentPatrolPoint (Variables|Default|GetPatrolPoint2))
    (Utilities|UpdatePatrolPointBB :!label _label)
    (elif (== OtherActor (Variables|Default|GetPatrolPoint2))
      (Variables|Default|SetCurrentPatrolPoint (Variables|Default|GetPatrolPoint1))
      (goto _label))))

(event EventTick
  (params (DeltaSeconds :type Float%20%28single-precision%29)))

(event Collision|EventHit
  (params (MyComp :type Primitive%20Component%20Object%20Reference) (Other :type Actor%20Object%20Reference) (OtherComp :type Primitive%20Component%20Object%20Reference) (bSelfMoved :type Boolean) (HitLocation :type Vector :default "0, 0, 0") (HitNormal :type Vector :default "0, 0, 0") (NormalImpulse :type Vector :default "0, 0, 0") (Hit :type Hit%20Result%20Structure%20%28by%20ref%29))
  (bind _mesh (Variables|Character|GetMesh))
  (Utilities|Casting|CastToBP_FirstPersonProjectile Other)
  (if (> (Variables|Default|GetEnemyHealth) 1)
    (Math|Integer|DecrementInt (Variables|Default|GetEnemyHealth)
      (:%20%20
        (Game|SpawnActorfromClass "/Game/StarterContent/Blueprints/Blueprint_Effect_Explosion.Blueprint_Effect_Explosion_C" (Transformation|GetActorTransform) "Undefined" 0 0)
        (Variables|/Script/Engine.CharacterMovementComponent|SetMaxWalkSpeed (Variables|Character|GetCharacterMovement) 7e+02)))
    (else
      (Variables|/Script/Engine.CharacterMovementComponent|SetMaxWalkSpeed (Variables|Character|GetCharacterMovement) 0.0)
      (Utilities|FlowControl|DoOnce false
        (:Completed
          (Components|Animation|PlayAnimation _mesh "/Game/Enemy/UndeadPack/SkeletonEnemy/Animations/Anim_Death.Anim_Death" false)
          (Collision|SetCollisionEnabled (Variables|Collision|GetCapsuleComponent) "NoCollision")
          (Collision|SetCollisionEnabled _mesh "NoCollision")
          (Utilities|FlowControl|Delay 1.5)
          (bind _asue_4asp_character (Utilities|Casting|CastToUe4ASP_Character (Game|GetPlayerCharacter 0)))
          (Math|Integer|IncrementInt (Variables|/Game/Character/Ue4ASP_Character.Ue4ASP_Character_C|GetTargetEliminated _asue_4asp_character)
            (:%20%20
              (Default|CheckGoal _asue_4asp_character)
              (Actor|DestroyActor))))))))

(fn ConstructionScript)